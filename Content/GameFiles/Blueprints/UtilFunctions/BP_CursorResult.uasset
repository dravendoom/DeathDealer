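; Utility Blueprint with one function that computes a spawn transform for something launched from a pawn toward the mouse cursor.
; The spawn location is the pawn's actor location.
; The spawn rotation comes from a complex Visibility trace under the player controller's cursor, taking the normalized pawn-to-hit direction as its X axis.
; Both points have Z zeroed, so the resulting aim stays on the horizontal plane.
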(fn NewFunction
  (params (pController :type Player%20Controller%20Object%20Reference) (pPawn :type Pawn%20Object%20Reference))
  (bind _returnvalue (Transformation|GetActorLocation pPawn))
  (bind _hitresult (Game|Player|GetHitResultUnderCursorbyChannel pController "TraceTypeQuery1" true))
  (bind _location (Collision|BreakHitResult _hitresult))
  (bind (_x _y _z) (Math|Vector|BreakVector _returnvalue))
  (bind (_x_2 _y_2 _z_2) (Math|Vector|BreakVector _location))
  (return _returnvalue (Math|Rotator|MakeRotfromX (Math|Vector|Normalize (- (Math|Vector|MakeVector _x_2 _y_2 (* _z_2 0.0)) (Math|Vector|MakeVector _x _y (* _z 0.0)))))))