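; BP_BloodSphere is a projectile attack for the first character that damages enemies it overlaps.
; On BeginPlay it sets its local-space projectile velocity from an initial velocity variable and rotates three Niagara effects to face the initial direction.
; Overlapping a BP_Enemy_Base applies fixed damage credited to player 0's character and controller, and the sphere is not destroyed by the hit.
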(event EventBeginPlay
  (Game|Components|ProjectileMovement|SetVelocityinLocalSpace (Variables|Default|GetProjectileMovement) (Variables|Default|GetInitialVeloctiy))
  (Transformation|SetRelativeRotation (Variables|Default|GetNiagara) (Math|Rotator|MakeRotfromX (Variables|Default|GetinitialDirection)) false false)
  (Transformation|SetRelativeRotation (Variables|Default|GetNiagara1) (Math|Rotator|MakeRotfromX (Variables|Default|GetinitialDirection)) false false)
  (Transformation|SetRelativeRotation (Variables|Default|GetNiagara2) (Math|Rotator|MakeRotfromX (Variables|Default|GetinitialDirection)) false false))

(event EventTick
  (params (DeltaSeconds :type Float%20%28single-precision%29)))

(event Collision|EventActorBeginOverlap
  (params (OtherActor :type Actor%20Object%20Reference))
  (bind _returnvalue (Game|GetPlayerCharacter 0))
  (bind _asbp_enemy_base (Utilities|Casting|CastToBP_Enemy_Base OtherActor))
  (Game|Damage|ApplyDamage _asbp_enemy_base 5e+01 (Pawn|GetController _returnvalue) _returnvalue))

(fn ConstructionScript)