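; BP_DefaultMan is the player's Paper2D vampire character, with axis movement, sprite flipping, a basic attack and XP leveling.
; Tick picks the idle, walk, run or attack flipbook from velocity and an attacking flag.
; After a short delay, attacks launch a BP_BloodSphere toward the cursor on the horizontal plane.
; XP thresholds set levels and notify the DeathDealer game mode; damage and death logic is disconnected.
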(event Custom|RecieveXP
  (params (XPRecieved :type Integer))
  ;[1 0.9114 0] LevelUpSystem
  (bind _output_get (Variables|Default|SetEXP (+ (Variables|Default|GetEXP) XPRecieved)))
  (if (> (Utilities|Array|FindItem (Variables|Default|GetXPArray) _output_get) 0)
    (bind _output_get_2 (Variables|Default|SetLevel (+ 1 (Utilities|Array|FindItem (Variables|Default|GetXPArray) _output_get))))
    (bind _asdeath_dealer (Utilities|Casting|CastToDeathDealer (Game|GetGameMode)))
    (Default|OnPlayerLevelUp _asdeath_dealer _output_get_2)))

(event EventBeginPlay
  ;[0.3611 0.5796 1] Setters
  (Variables|Default|SetHealth 100)
  (Variables|Default|SetEXP 0)
  (Variables|Default|SetLevel 1))

(event Game|Damage|EventAnyDamage
  (params (Damage :type Float%20%28single-precision%29) (DamageType :type Damage%20Type%20Object%20Reference) (InstigatedBy :type Controller%20Object%20Reference) (DamageCauser :type Actor%20Object%20Reference))
  ;[1 0 0.6349] DamageAndDeath
)

(event EventTick
  (params (DeltaSeconds :type Float%20%28single-precision%29))
  (bind _flipbook (Variables|Default|GetFlipBook))
  (bind _charactermovement (Variables|Character|GetCharacterMovement))
  (bind _updatedprimitive (Variables|/Script/Engine.MovementComponent|GetUpdatedPrimitive _charactermovement))
  (bind _returnvalue (Transformation|GetComponentVelocity _updatedprimitive))
  (bind _returnvalue_2 (Math|Vector|VectorLength _returnvalue))
  ;[1 0.4678 0.4969 0.3608] Movement Animations
  (if (Variables|Default|GetisAttacking)
    (Sprite|SetFlipbook (Variables|Default|GetFlipBook) "/Game/GameFiles/Sprites/Characters/VampireGirl/Vampire_Attack.Vampire_Attack")
    (elif (> _returnvalue_2 0.0)
      (if (> _returnvalue_2 5e+02)
        (Sprite|SetFlipbook _flipbook "/Game/GameFiles/Sprites/Characters/VampireGirl/Vampire_Run.Vampire_Run")
        (else
          (Sprite|SetFlipbook _flipbook "/Game/GameFiles/Sprites/Characters/VampireGirl/Vampire_Walk.Vampire_Walk")))
      (else
        (Sprite|SetFlipbook _flipbook "/Game/GameFiles/Sprites/Characters/VampireGirl/Vampire_Idle.Vampire_Idle")))))

(event Input|ActionEvents|InputActionBasicAttack
  (params (Key :type Key%20Structure :default "None"))
  (bind _returnvalue (Game|Player|GetPlayerPawn 0))
  (bind _returnvalue_2 (Game|GetPlayerController 0))
  (bind _hitresult (Game|Player|GetHitResultUnderCursorbyChannel _returnvalue_2 "TraceTypeQuery1" true))
  (bind _returnvalue_3 (Transformation|GetActorLocation _returnvalue))
  (bind (_x _y _z) (Math|Vector|BreakVector _returnvalue_3))
  (bind _location (Collision|BreakHitResult _hitresult))
  (bind (_x_2 _y_2 _z_2) (Math|Vector|BreakVector _location))
  (bind _returnvalue_4 (* _z 0.0))
  (bind _returnvalue_5 (Math|Vector|MakeVector _x _y _returnvalue_4))
  (bind _returnvalue_6 (* _z_2 0.0))
  (bind _returnvalue_7 (Math|Vector|MakeVector _x_2 _y_2 _returnvalue_6))
  (bind _returnvalue_8 (- _returnvalue_7 _returnvalue_5))
  (bind _returnvalue_9 (Math|Vector|Normalize _returnvalue_8))
  ;[1 0.04151 0.05809] BasicAttacck2
  (:Pressed
    (Variables|Default|SetisAttacking true)
    (Utilities|FlowControl|Delay 0.4)
    (bind _returnvalue_10 (Game|SpawnActorfromClass "/Game/GameFiles/Blueprints/Characters/First_Char/Attack/BP_BloodSphere.BP_BloodSphere_C" (Math|Transform|MakeTransform _returnvalue_3 (Math|Rotator|MakeRotfromX _returnvalue_9)) "Undefined" "MultiplyWithRoot" 0 0))
    (Variables|/Game/GameFiles/Blueprints/Characters/First_Char/Attack/BP_BloodSphere.BP_BloodSphere_C|SetInitialVeloctiy _returnvalue_10 (* _returnvalue_9 25.0))
    (Variables|Default|SetisAttacking false)))

(event Input|AxisEvents|InputAxisFrontalMovement
  (params (AxisValue :type Float%20%28single-precision%29))
  ;[0.4342 0.4287 1 0.3608] Up And Down Movement
  (Pawn|Input|AddMovementInput (Transformation|GetActorRightVector) AxisValue false))

(event Input|AxisEvents|InputAxisSideMovement
  (params (AxisValue :type Float%20%28single-precision%29))
  ;[0.4342 0.4287 1 0.3608] Left And Right Movement
  (Pawn|Input|AddMovementInput (Transformation|GetActorForwardVector) AxisValue false)
  (if (> AxisValue 0.0)
    (Transformation|SetRelativeScale3D (Variables|Default|GetPaperSprite) "1.000000,1.000000,1.000000")
    (else
      (Transformation|SetRelativeScale3D (Variables|Default|GetPaperSprite) "-1.000000,1.000000,1.000000"))))

(fn ConstructionScript)