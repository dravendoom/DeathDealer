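; BP_SelectItem is an actor that exercises its Inventory's random loot picks, printing results as debug text without granting items.
; From BeginPlay, a delayed loop checks the rarity for NoDrop or Normal, prints rarity and item, then calls Reroll.
; Magic, Rare and Legendary checks are disconnected, so any other rarity takes the Magic pick.
; PickRarity is called separately per check and print, so printed rarity can differ from the branch taken.
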(event OnInventoryFull(Inventory)
  (params (Item :type Item%20Data%20Struct%20Structure%20%28by%20ref%29)))

(event Custom|reroll
  (bind _inventory (Variables|Default|GetInventory))
  (bind _inventory_2 (Variables|Default|GetInventory))
  (bind _returnvalue (Class|Inventory|PickRarity _inventory))
  (bind _returnvalue_2 (Utilities|String|EnumtoString _returnvalue))
  (Utilities|FlowControl|Delay 5e+02)
  (if (Utilities|Enum|Equal(Enum) "NoDrop" _returnvalue_2)
    (Development|PrintString "NODROP")
    (elif (Utilities|Enum|Equal(Enum) "Normal" _returnvalue_2)
      (Development|PrintString (Utilities|String|Append "Rarity: " _returnvalue_2 " |" "Item: " (Utilities|String|EnumtoString (Class|Inventory|PickNormalItem _inventory_2))))
      (elif true
        (Development|PrintString (Utilities|String|Append "Rarity: " _returnvalue_2 " |" "Item: " (Utilities|String|EnumtoString (Class|Inventory|PickMagicItem _inventory_2))))
        (elif true
          (Development|PrintString (Utilities|String|Append "Rarity: " _returnvalue_2 " |" "Item: " (Utilities|String|EnumtoString (Class|Inventory|PickRareItem _inventory_2))))
          (elif true
            (Development|PrintString (Utilities|String|Append "Rarity: " _returnvalue_2 " |" "Item: " (Utilities|String|EnumtoString (Class|Inventory|PickLegendaryItem _inventory_2))))
            (else
              (Development|PrintString "False")))))))
  (CallFunction|Reroll))

(event EventBeginPlay
  (bind _inventory (Variables|Default|GetInventory))
  (bind _inventory_2 (Variables|Default|GetInventory))
  (bind _returnvalue (Class|Inventory|PickRarity _inventory))
  (bind _returnvalue_2 (Utilities|String|EnumtoString _returnvalue))
  (Utilities|FlowControl|Delay 5e+02)
  (if (Utilities|Enum|Equal(Enum) "NoDrop" _returnvalue_2)
    (Development|PrintString "NODROP")
    (elif (Utilities|Enum|Equal(Enum) "Normal" _returnvalue_2)
      (Development|PrintString (Utilities|String|Append "Rarity: " _returnvalue_2 " |" "Item: " (Utilities|String|EnumtoString (Class|Inventory|PickNormalItem _inventory_2))))
      (elif true
        (Development|PrintString (Utilities|String|Append "Rarity: " _returnvalue_2 " |" "Item: " (Utilities|String|EnumtoString (Class|Inventory|PickMagicItem _inventory_2))))
        (elif true
          (Development|PrintString (Utilities|String|Append "Rarity: " _returnvalue_2 " |" "Item: " (Utilities|String|EnumtoString (Class|Inventory|PickRareItem _inventory_2))))
          (elif true
            (Development|PrintString (Utilities|String|Append "Rarity: " _returnvalue_2 " |" "Item: " (Utilities|String|EnumtoString (Class|Inventory|PickLegendaryItem _inventory_2))))
            (else
              (Development|PrintString "False")))))))
  (CallFunction|Reroll))

(event Collision|EventActorBeginOverlap
  (params (OtherActor :type Actor%20Object%20Reference)))

(event EventTick
  (params (DeltaSeconds :type Float%20%28single-precision%29)))

(fn ConstructionScript)