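; BP_AddItems applies one item's stat bonuses to the player character, BP_DefaultMan, when play begins.
; It reads the hardcoded "Cap" row from an item data table and prints its name, rarity and description.
; It then loops over the row's Stats map, routing each stat type to the character's health, damage multiplier or movement speed add function.
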(event EventBeginPlay
  (bind _asbp_default_man (Utilities|Casting|CastToBP_DefaultMan (Game|GetPlayerCharacter 0)))
  (Variables|Default|SetBP_DefaultMan _asbp_default_man)
  (bind _returnvalue (Utilities|GetDataTableRow (Variables|Default|GetItemDataTable) "Cap")
    (:then
      (Development|PrintString (Utilities|String|Append (.ItemName (Utilities|Struct|BreakItemDataStruct _returnvalue)) (.ItemRarity (Utilities|Struct|BreakItemDataStruct _returnvalue)) (.ItemDescription (Utilities|Struct|BreakItemDataStruct _returnvalue))))
      (bind _keys (Utilities|Map|Keys (.Stats (Utilities|Struct|BreakItemDataStruct _returnvalue))))
      (for _array_element _keys
        (switch name _array_element
          (:Health
            (Default|AddHealth (Variables|Default|GetBP_DefaultMan) (Math|Float|Truncate (.Value (Utilities|Map|Find (.Stats (Utilities|Struct|BreakItemDataStruct _returnvalue)) _array_element)))))
          (:DamageMulti
            (Default|AddDamMult (Variables|Default|GetBP_DefaultMan) (.Value (Utilities|Map|Find (.Stats (Utilities|Struct|BreakItemDataStruct _returnvalue)) _array_element))))
          (:MovementSpeed
            (Default|AddMovement (Variables|Default|GetBP_DefaultMan) (.Value (Utilities|Map|Find (.Stats (Utilities|Struct|BreakItemDataStruct _returnvalue)) _array_element)))))))))

(fn ConstructionScript)