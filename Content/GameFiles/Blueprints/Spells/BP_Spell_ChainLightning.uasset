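; Chain lightning spell actor that auto-casts around the player on a looping timer scaled by the player's cooldown stat.
; Each cast damages the pawn within range of the player nearest the last stored origin, using the player's damage multiplier.
; It then repeats overlap searches from each hit point for the chain count, drawing debug lines as bolts.
; Searches ignore only the player, so already-hit pawns remain valid targets.
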(event Custom|ChainLightning
  (bind _returnvalue (Game|Player|GetPlayerPawn 0))
  (bind _returnvalue_2 (Game|GetPlayerCharacter 0))
  (bind _array (Utilities|Array|MakeArray "ObjectTypeQuery3"))
  (bind _player_reference (Variables|Default|GetPlayer%20Reference))
  (bind (_outactors _returnvalue_3) (Collision|SphereOverlapActors (Transformation|GetActorLocation (Game|GetPlayerCharacter 0)) (Variables|Default|GetAoE_0) _array 0 (Utilities|Array|MakeArray _returnvalue_2)))
  (if _returnvalue_3
    (Variables|Default|SetNewOriginPoint (Transformation|GetActorLocation (.ReturnValue (Actor|FindNearestActor (Variables|Default|GetNewOriginPoint) _outactors))))
    (bind _output_get (Variables|Default|SetActualDamage (* (Variables|Default|GetBaseDamage) (Variables|/Game/GameFiles/Blueprints/Characters/First_Char/BP_DefaultMan.BP_DefaultMan_C|GetPlayerMoreDamMul _player_reference))))
    (Game|Damage|ApplyDamage (.ReturnValue (Actor|FindNearestActor (Variables|Default|GetNewOriginPoint) _outactors)) _output_get 0 _returnvalue_2)
    (for _index (range 0 (+ (Variables|/Game/GameFiles/Blueprints/Characters/First_Char/BP_DefaultMan.BP_DefaultMan_C|GetChains _player_reference) (Variables|Default|GetChains_0)))
      (bind (_outactors_2 _returnvalue_4) (Collision|SphereOverlapActors (Variables|Default|GetNewOriginPoint) (Variables|Default|GetAoE_0) _array 0 (Utilities|Array|MakeArray _returnvalue)))
      (if _returnvalue_4
        (bind _output_get_2 (Variables|Default|SetNewOriginPoint (Transformation|GetActorLocation (.ReturnValue (Actor|FindNearestActor (Variables|Default|GetNewOriginPoint) _outactors_2)))))
        (Rendering|Debug|DrawDebugLine (stale _output_get_3) _output_get_2 "(R=0.000000,G=0.709213,B=1.000000,A=1.000000)" 0.25 4.0)
        (bind _output_get_3 (Variables|Default|SetPreviousLocation _output_get_2))
        (Game|Damage|ApplyDamage (.ReturnValue (Actor|FindNearestActor (Variables|Default|GetNewOriginPoint) _outactors_2)) (Variables|Default|GetActualDamage) 0 _returnvalue)))))

(event EventBeginPlay
  (bind _returnvalue (Game|GetPlayerCharacter 0))
  (bind _asbp_default_man (Utilities|Casting|CastToBP_DefaultMan _returnvalue))
  (Variables|Default|SetPlayer%20Reference _asbp_default_man)
  (Variables|Default|SetNewOriginPoint (Transformation|GetActorLocation _returnvalue))
  (bind _returnvalue_2 (Utilities|Time|SetTimerbyEvent (delegate Custom|ChainLightning) (* (Variables|/Game/GameFiles/Blueprints/Characters/First_Char/BP_DefaultMan.BP_DefaultMan_C|GetPlayerCooldown (Variables|Default|GetPlayer%20Reference)) (Variables|Default|GetCooldown_0)) true))
  (Variables|Default|SetTimer _returnvalue_2))

(event Collision|EventActorBeginOverlap
  (params (OtherActor :type Actor%20Object%20Reference)))

(event EventTick
  (params (DeltaSeconds :type Float%20%28single-precision%29)))

(fn ConstructionScript)