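; Fireball spell that auto-casts on a looping timer, with its interval scaled by the player's cooldown stat.
; Each cast spawns an explosion at GetHitLocation and applies damage to sphere-overlapped actors other than the player, then re-sets the timer.
; Radius and damage scale with stats read from BP_DefaultMan.
; A multi-explosion CastCascade variant with fixed damage exists behind a hard-coded false branch.
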(event Custom|Cast_FireBall
  (bind _returnvalue (Game|GetPlayerCharacter 0))
  (bind _aoe_0 (Variables|Default|GetAoE_0))
  (bind _basedamage (Variables|Default|GetBaseDamage))
  (bind _as_bp_default_man (Variables|Default|GetAs%20BP%20Default%20Man))
  (bind _playeraoe (Variables|/Game/GameFiles/Blueprints/Characters/First_Char/BP_DefaultMan.BP_DefaultMan_C|GetPlayerAoE _as_bp_default_man))
  (bind _playermoredammul (Variables|/Game/GameFiles/Blueprints/Characters/First_Char/BP_DefaultMan.BP_DefaultMan_C|GetPlayerMoreDamMul _as_bp_default_man))
  (bind _returnvalue_2 (* _basedamage _playermoredammul))
  (bind _returnvalue_3 (* _aoe_0 _playeraoe))
  (if false
    (CallFunction|CastCascade)
    (else
      (bind _output_get (Variables|Default|SetspellCastLocation (Utilities|GetHitLocation)))
      (Effects|SpawnEmitteratLocation "/Game/StarterContent/Particles/P_Explosion.P_Explosion" _output_get "0, 0, 0" (Math|Conversions|ToVector(Float) (.X (Math|Vector|BreakVector (Math|Conversions|ToVector(Float) (/ _returnvalue_3 1.5e+02))))))
      (bind _outactors (Collision|SphereOverlapActors (Variables|Default|GetspellCastLocation) _returnvalue_3 (Variables|Default|GetObject%20Types_1) 0 (Utilities|Array|MakeArray _returnvalue)))
      (for _array_element _outactors
        (bind _output_get_2 (Variables|Default|SetFullDam _returnvalue_2))
        (Game|Damage|ApplyDamage _array_element _output_get_2 0 _returnvalue)
        (Development|PrintString (Utilities|String|Append "Base Damage:" (Utilities|String|ToString(Float) _returnvalue_2))))
      (CallFunction|Cooldownevent))))

(event Custom|CastCascade
  (bind _aoe_0 (Variables|Default|GetAoE_0))
  (bind _as_bp_default_man (Variables|Default|GetAs%20BP%20Default%20Man))
  (bind _playeraoe (Variables|/Game/GameFiles/Blueprints/Characters/First_Char/BP_DefaultMan.BP_DefaultMan_C|GetPlayerAoE _as_bp_default_man))
  (bind _returnvalue (* _playeraoe _aoe_0))
  (bind _output_get (Variables|Default|SetspellCastLocation (Utilities|GetHitLocation)))
  (for _index (range 0 25)
    (bind _output_get_2 (Variables|Default|SetRandomPoint (Math|Random|RandomPointinBoundingBox _output_get (Math|Vector|MakeVector _returnvalue _returnvalue _returnvalue))))
    (bind _outactors (Collision|SphereOverlapActors _output_get_2 _returnvalue (Variables|Default|GetObject%20Types_1) 0 (Utilities|Array|MakeArray (Game|GetPlayerCharacter 0))))
    (Effects|SpawnEmitteratLocation "/Game/StarterContent/Particles/P_Explosion.P_Explosion" _output_get_2 "0, 0, 0" "0.500000,0.500000,0.500000")
    (for _array_element _outactors
      (Game|Damage|ApplyDamage _array_element 1e+02 0 (Game|GetPlayerCharacter 0)))))

(event Custom|cooldownevent
  (Utilities|Time|SetTimerbyEvent (delegate Custom|Cast_FireBall) (* (Variables|Default|GetCooldown_0) (Variables|/Game/GameFiles/Blueprints/Characters/First_Char/BP_DefaultMan.BP_DefaultMan_C|GetPlayerCooldown (Variables|Default|GetAs%20BP%20Default%20Man))) true))

(event EventBeginPlay
  (bind _asbp_default_man (Utilities|Casting|CastToBP_DefaultMan (Game|GetPlayerCharacter 0)))
  (Variables|Default|SetAs%20BP%20Default%20Man _asbp_default_man)
  (Utilities|Time|SetTimerbyEvent (delegate Custom|Cast_FireBall) (* (Variables|Default|GetCooldown_0) (Variables|/Game/GameFiles/Blueprints/Characters/First_Char/BP_DefaultMan.BP_DefaultMan_C|GetPlayerCooldown (Variables|Default|GetAs%20BP%20Default%20Man))) true))

(fn ConstructionScript)