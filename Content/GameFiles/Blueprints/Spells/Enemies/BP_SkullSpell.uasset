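; BP_SkullSpell is an enemy spell projectile launched toward the player's position at the moment it spawns.
; On BeginPlay it casts its owner to BP_Enemy_Base and takes a flattened, horizontal direction from that enemy to player 0.
; That direction rotates the Niagara effect and, scaled by ProjSpeed, is set as the ProjectileMovement local-space velocity.
; It has no homing or overlap logic of its own.
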(event EventBeginPlay
  (bind _returnvalue (Game|GetPlayerCharacter 0))
  (bind _returnvalue_2 (Transformation|GetActorLocation _returnvalue))
  (bind (_x _y _z) (Math|Vector|BreakVector _returnvalue_2))
  (bind _asbp_enemy_base (Utilities|Casting|CastToBP_Enemy_Base (Components|GetOwner)))
  (Transformation|SetWorldRotation (Variables|Default|GetNiagara) (Math|Rotator|MakeRotfromX (Math|Vector|GetUnitDirection(Vector) (Math|Vector|MakeVector (.X (Math|Vector|BreakVector (Transformation|GetActorLocation _asbp_enemy_base))) (.Y (Math|Vector|BreakVector (Transformation|GetActorLocation _asbp_enemy_base))) (* (.Z (Math|Vector|BreakVector (Transformation|GetActorLocation _asbp_enemy_base))) 0.0)) (Math|Vector|MakeVector _x _y (* _z 0.0)))) false false)
  (Game|Components|ProjectileMovement|SetVelocityinLocalSpace (Variables|Default|GetProjectileMovement) (* (Math|Vector|GetUnitDirection(Vector) (Math|Vector|MakeVector (.X (Math|Vector|BreakVector (Transformation|GetActorLocation _asbp_enemy_base))) (.Y (Math|Vector|BreakVector (Transformation|GetActorLocation _asbp_enemy_base))) (* (.Z (Math|Vector|BreakVector (Transformation|GetActorLocation _asbp_enemy_base))) 0.0)) (Math|Vector|MakeVector _x _y (* _z 0.0))) (Variables|Default|GetprojSpeed))))

(event Collision|EventActorBeginOverlap
  (params (OtherActor :type Actor%20Object%20Reference)))

(event EventTick
  (params (DeltaSeconds :type Float%20%28single-precision%29)))

(fn ConstructionScript)