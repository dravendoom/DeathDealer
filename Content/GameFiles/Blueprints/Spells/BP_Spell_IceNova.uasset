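; Auto-cast Ice Nova spell that periodically releases an expanding damage area at its owner's location.
; A timer scaled by the player's cooldown stat moves the capsule and effect to the owner and starts NovaTimeLine.
; The timeline grows the capsule radius to the player-scaled AoE, then disables collision and restarts the cooldown.
; Actor overlaps apply damage scaled by the player's damage multiplier, credited to the player.
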(event Custom|CastIceNova
  (bind _capsule (Variables|Default|GetCapsule))
  (Transformation|SetWorldLocation _capsule (Transformation|GetActorLocation (Components|GetOwner)) false false)
  (Collision|SetCollisionEnabled _capsule "QueryOnly")
  (Components|Timeline|PlayfromStart (Variables|Default|GetNovaTimeLine)))

(event Custom|Trigger%20Cooldown
  (bind _returnvalue (Utilities|Time|SetTimerbyEvent (delegate Custom|CastIceNova) (* (Variables|/Game/GameFiles/Blueprints/Characters/First_Char/BP_DefaultMan.BP_DefaultMan_C|GetPlayerCooldown (Variables|Default|GetPlayer%20Reference)) (Variables|Default|GetCooldown))))
  (Variables|Default|SettimerHandle _returnvalue))

(event EventBeginPlay
  (bind _asbp_default_man (Utilities|Casting|CastToBP_DefaultMan (Game|GetPlayerCharacter 0)))
  (Variables|Default|SetPlayer%20Reference _asbp_default_man)
  (Components|Activation|SetActive (Variables|Default|GetIceNova) false false)
  (bind _returnvalue (Utilities|Time|SetTimerbyEvent (delegate Custom|CastIceNova) (* (Variables|/Game/GameFiles/Blueprints/Characters/First_Char/BP_DefaultMan.BP_DefaultMan_C|GetPlayerCooldown (Variables|Default|GetPlayer%20Reference)) (Variables|Default|GetCooldown))))
  (Variables|Default|SettimerHandle _returnvalue))

(event EventTick
  (params (DeltaSeconds :type Float%20%28single-precision%29)))

(event Collision|EventActorBeginOverlap
  (params (OtherActor :type Actor%20Object%20Reference))
  (bind _returnvalue (Game|GetPlayerCharacter 0))
  (Game|Damage|ApplyDamage OtherActor (* (Variables|/Game/GameFiles/Blueprints/Characters/First_Char/BP_DefaultMan.BP_DefaultMan_C|GetPlayerMoreDamMul (Variables|Default|GetPlayer%20Reference)) (Variables|Default|GetBaseDamage)) (Pawn|GetController _returnvalue) _returnvalue))

(fn ConstructionScript)