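; Flame Front spell caster that automatically and repeatedly fires a fan of BP_Spell_FlameFront actors for the player.
; On BeginPlay it derives a cooldown from BP_DefaultMan and a base value, then starts a looping timer.
; Each cast gets spawn location and rotation from the player's controller and pawn, then spawns a center projectile.
; An index-parity loop adds yaw-offset copies on alternating sides, accumulating angles per side and printing debug values.
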(event Custom|CastFlameFront
  (bind (_spawnlocation _spawnrotation) (CallFunction|NewFunction (Game|GetPlayerController 0) (Game|Player|GetPlayerPawn 0)))
  (bind _output_get (Variables|Default|SetinitialRotation _spawnrotation))
  (Game|SpawnActorfromClass "/Game/GameFiles/Blueprints/Spells/FlameFront/BP_Spell_FlameFront.BP_Spell_FlameFront_C" (Math|Transform|MakeTransform _spawnlocation _output_get) "Undefined" "MultiplyWithRoot" 0 0)
  (Variables|Default|SetsetNewAngle 0.0)
  (for _index (range 1 2)
    (if (== (Math|Integer|%(Integer) _index 2) 0)
      (bind _output_get_2 (Variables|Default|SetsetNewAngle (- (Variables|Default|GetnegativeSaveAngle) 3e+01)))
      (Development|PrintString (Utilities|String|Append "Negative: " (Utilities|String|ToString(Float) (Variables|Default|GetnegativeSaveAngle))))
      (Game|SpawnActorfromClass "/Game/GameFiles/Blueprints/Spells/FlameFront/BP_Spell_FlameFront.BP_Spell_FlameFront_C" (Math|Transform|MakeTransform _spawnlocation (Math|Rotator|MakeRotator (.Roll (Math|Rotator|BreakRotator _output_get)) (.Pitch (Math|Rotator|BreakRotator _output_get)) (+ (.Yaw (Math|Rotator|BreakRotator _output_get)) _output_get_2))) "Undefined" "MultiplyWithRoot" 0 0)
      (Variables|Default|SetnegativeSaveAngle _output_get_2)
      (Variables|Default|SetsetNewAngle 0.0)
      (else
        (bind _output_get_3 (Variables|Default|SetsetNewAngle (+ 3e+01 (Variables|Default|GetpositiveSaveAngle))))
        (Development|PrintString (Utilities|String|Append "Positive: " (Utilities|String|ToString(Float) (Variables|Default|GetpositiveSaveAngle))))
        (Game|SpawnActorfromClass "/Game/GameFiles/Blueprints/Spells/FlameFront/BP_Spell_FlameFront.BP_Spell_FlameFront_C" (Math|Transform|MakeTransform _spawnlocation (Math|Rotator|MakeRotator (.Roll (Math|Rotator|BreakRotator _output_get)) (.Pitch (Math|Rotator|BreakRotator _output_get)) (+ (.Yaw (Math|Rotator|BreakRotator _output_get)) _output_get_3))) "Undefined" "MultiplyWithRoot" 0 0)
        (Variables|Default|SetpositiveSaveAngle _output_get_3)
        (Variables|Default|SetsetNewAngle 0.0))))
  (Variables|Default|SetnegativeSaveAngle 0.0)
  (Variables|Default|SetpositiveSaveAngle 0.0))

(event EventBeginPlay
  (bind _asbp_default_man (Utilities|Casting|CastToBP_DefaultMan (Game|GetPlayerCharacter 0)))
  (bind _output_get (Variables|Default|SetAs%20BP%20Default%20Man _asbp_default_man))
  (bind _truecooldown (CallFunction|CooldownCalc _output_get 2.0))
  (Utilities|Time|SetTimerbyEvent (delegate Custom|CastFlameFront) _truecooldown true))

(fn ConstructionScript
  (|CallParentFunction))