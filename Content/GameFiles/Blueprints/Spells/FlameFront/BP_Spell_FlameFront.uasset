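; BP_Spell_FlameFront is a short-lived flame spell projectile that bursts into a flame blast when it hits an enemy.
; On BeginPlay it moves forward in local space and destroys itself after a brief delay.
; The first sphere overlap with a BP_Enemy_Base, guarded by a one-shot flag, spawns BP_Spell_FlameBlast at its location and destroys the projectile.
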(event OnComponentBeginOverlap(Sphere)
  (params (OverlappedComponent :type Primitive%20Component%20Object%20Reference) (OtherActor :type Actor%20Object%20Reference) (OtherComp :type Primitive%20Component%20Object%20Reference) (OtherBodyIndex :type Integer) (bFromSweep :type Boolean) (SweepResult :type Hit%20Result%20Structure%20%28by%20ref%29))
  (Utilities|Casting|CastToBP_Enemy_Base OtherActor)
  (if (not (Variables|Default|GetOverlapped))
    (Variables|Default|SetOverlapped true)
    (Game|SpawnActorfromClass "/Game/GameFiles/Blueprints/Spells/FlameFront/BP_Spell_FlameBlast.BP_Spell_FlameBlast_C" (Math|Transform|MakeTransform (Transformation|GetActorLocation self)) "Undefined" "MultiplyWithRoot" 0 0)
    (Actor|DestroyActor)))

(event Collision|EventActorBeginOverlap
  (params (OtherActor :type Actor%20Object%20Reference)))

(event EventTick
  (params (DeltaSeconds :type Float%20%28single-precision%29)))

(event EventBeginPlay
  (Game|Components|ProjectileMovement|SetVelocityinLocalSpace (Variables|Default|GetProjectileMovement) "250.000000,0.000000,0.000000")
  (Utilities|FlowControl|Delay 1.33)
  (Actor|DestroyActor))

(fn ConstructionScript
  (|CallParentFunction))