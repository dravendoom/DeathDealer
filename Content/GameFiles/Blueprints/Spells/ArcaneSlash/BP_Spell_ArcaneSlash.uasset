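; BP_Spell_ArcaneSlash is an Arcane Slash spell that repeatedly auto-casts BP_ASlash actors for the player.
; BeginPlay starts a looping timer, with its interval set by the spell cooldown times the player's cooldown.
; Each cast gets its spawn transform from NewFunction and scales the slash and its Niagara effect by StrikeNum.
; StrikeNum increments after each cast, but resets to 1 whenever the result is three or less.
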(event Custom|CastFlameFront
  (bind (_spawnlocation _spawnrotation) (CallFunction|NewFunction (Game|GetPlayerController 0) (Game|Player|GetPlayerPawn 0)))
  (bind _output_get (Variables|Default|SetSpawn%20Rotation _spawnrotation))
  (bind _returnvalue (Game|SpawnActorfromClass "/Game/GameFiles/Blueprints/Spells/ArcaneSlash/BP_ASlash.BP_ASlash_C" (Math|Transform|MakeTransform _spawnlocation _output_get (* (Variables|Default|GetscaleSetter) (Variables|Default|GetstrikeNum))) "Undefined" "MultiplyWithRoot" 0 0))
  (Transformation|SetRelativeScale3D (Variables|/Game/GameFiles/Blueprints/Spells/ArcaneSlash/BP_ASlash.BP_ASlash_C|GetNiagara _returnvalue) (* (Variables|Default|GetscaleSetter) (Variables|Default|GetstrikeNum)))
  (bind _output_get_2 (Variables|Default|SetstrikeNum (+ (Variables|Default|GetstrikeNum) 1)))
  (if (<= _output_get_2 3)
    (Variables|Default|SetstrikeNum 1)))

(event EventBeginPlay
  (bind _asbp_default_man (Utilities|Casting|CastToBP_DefaultMan (Game|GetPlayerCharacter 0)))
  (Variables|Default|SetAs%20BP%20Default%20Man _asbp_default_man)
  (Utilities|Time|SetTimerbyEvent (delegate Custom|CastFlameFront) (* (Variables|/Game/GameFiles/Blueprints/Characters/First_Char/BP_DefaultMan.BP_DefaultMan_C|GetplayerCooldown (Variables|Default|GetAs%20BP%20Default%20Man)) (Variables|Default|GetCooldown)) true))

(event Collision|EventActorBeginOverlap
  (params (OtherActor :type Actor%20Object%20Reference)))

(event EventTick
  (params (DeltaSeconds :type Float%20%28single-precision%29)))

(fn ConstructionScript
  (|CallParentFunction))