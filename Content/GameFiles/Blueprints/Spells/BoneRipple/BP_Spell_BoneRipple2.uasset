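; BP_Spell_BoneRipple2 is a short-lived Bone Ripple spell projectile that damages enemies it overlaps.
; On spawn it multiplies its base damage by the player's PlayerCooldown value, sets a forward local velocity, and destroys itself after a brief delay.
; Each overlapped BP_Enemy_Base receives that damage with the player character as causer, and hits do not end the projectile.
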(event EventBeginPlay
  (bind _asbp_default_man (Utilities|Casting|CastToBP_DefaultMan (Game|GetPlayerCharacter 0)))
  (Variables|Default|SetPlayerCharacter _asbp_default_man)
  (bind _output_get (Variables|Default|SetTotal%20Damage (* (Variables|Default|GetBase%20Damage) (Variables|/Game/GameFiles/Blueprints/Characters/First_Char/BP_DefaultMan.BP_DefaultMan_C|GetplayerCooldown _asbp_default_man))))
  (Game|Components|ProjectileMovement|SetVelocityinLocalSpace (Variables|Default|GetProjectileMovement) "250.000000,0.000000,0.000000")
  (Utilities|FlowControl|Delay 0.66)
  (Actor|DestroyActor))

(event Collision|EventActorBeginOverlap
  (params (OtherActor :type Actor%20Object%20Reference))
  (bind _asbp_enemy_base (Utilities|Casting|CastToBP_Enemy_Base OtherActor))
  (Game|Damage|ApplyDamage _asbp_enemy_base (stale EventBeginPlay _output_get) 0 (Game|GetPlayerCharacter 0)))

(event EventTick
  (params (DeltaSeconds :type Float%20%28single-precision%29)))

(fn ConstructionScript
  (|CallParentFunction))