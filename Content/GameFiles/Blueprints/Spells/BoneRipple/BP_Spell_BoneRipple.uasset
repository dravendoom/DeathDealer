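; Bone Ripple spell projectile that bursts into rings of secondary BP_Spell_BoneRipple2 actors.
; On BeginPlay it prints and applies DirectionVector as local-space velocity, then runs two timed bursts at its current location.
; Each burst steps an accumulated yaw in 60-degree increments; the first loops past a full circle, stacking spawns, and the second restarts from an offset angle.
; The projectile destroys itself after the second burst.
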(event EventBeginPlay
  (bind _directionvector (Variables|Default|GetDirectionVector))
  (Development|PrintString (Utilities|String|Append "Speed + Direction Vector: " (Utilities|String|ToString(Vector) _directionvector)))
  (Game|Components|ProjectileMovement|SetVelocityinLocalSpace (Variables|Default|GetProjectileMovement) _directionvector)
  (Utilities|FlowControl|Delay 0.66)
  (for _index (range 0 12)
    (bind _output_get (Variables|Default|SetArc (+ (Variables|Default|GetArc) 6e+01)))
    (Game|SpawnActorfromClass "/Game/GameFiles/Blueprints/Spells/BoneRipple/BP_Spell_BoneRipple2.BP_Spell_BoneRipple2_C" (Math|Transform|MakeTransform (Transformation|GetWorldLocation (Variables|Default|GetDefaultSceneRoot)) (Math|Rotator|MakeRotator 0.0 0.0 _output_get)) "Undefined" "MultiplyWithRoot" 0 0))
  (Variables|Default|SetArc 35.0)
  (Utilities|FlowControl|Delay 0.33)
  (for _index_2 (range 0 6)
    (bind _output_get_2 (Variables|Default|SetArc (+ (Variables|Default|GetArc) 6e+01)))
    (Game|SpawnActorfromClass "/Game/GameFiles/Blueprints/Spells/BoneRipple/BP_Spell_BoneRipple2.BP_Spell_BoneRipple2_C" (Math|Transform|MakeTransform (Transformation|GetWorldLocation (Variables|Default|GetDefaultSceneRoot)) (Math|Rotator|MakeRotator 0.0 0.0 _output_get_2)) "Undefined" "MultiplyWithRoot" 0 0))
  (Actor|DestroyActor)
  (Variables|Default|SetprojectileHit false))

(event EventTick
  (params (DeltaSeconds :type Float%20%28single-precision%29))
  (|CallParentFunction DeltaSeconds) ; This node is disabled and will not be called.\nDrag off pins to build functionality.
)

(fn ConstructionScript
  (|CallParentFunction))