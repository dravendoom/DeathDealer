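; Spell spawner actor for the Bone Ripple spell, automatically casting it toward the mouse cursor at a repeating interval.
; On BeginPlay it starts a looping timer timed by the player's PlayerCooldown multiplied by its own Cooldown.
; Each tick spawns a BP_Spell_BoneRipple at the player pawn, rotated toward the cursor's visibility-trace hit.
; It sets that projectile's DirectionVector to the height-flattened aim direction scaled by a fixed magnitude.
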(event Custom|BoneRipple
  (bind _returnvalue (Game|Player|GetPlayerPawn 0))
  (bind _returnvalue_2 (Game|GetPlayerController 0))
  (bind _returnvalue_3 (Transformation|GetActorLocation _returnvalue))
  (bind _hitresult (Game|Player|GetHitResultUnderCursorbyChannel _returnvalue_2 "TraceTypeQuery1" true))
  (bind _location (Collision|BreakHitResult _hitresult))
  (bind (_x _y _z) (Math|Vector|BreakVector _returnvalue_3))
  (bind (_x_2 _y_2 _z_2) (Math|Vector|BreakVector _location))
  (bind _returnvalue_4 (* _z 0.0))
  (bind _returnvalue_5 (Math|Vector|MakeVector _x _y _returnvalue_4))
  (bind _returnvalue_6 (* _z_2 0.0))
  (bind _returnvalue_7 (Math|Vector|MakeVector _x_2 _y_2 _returnvalue_6))
  (bind _returnvalue_8 (- _returnvalue_7 _returnvalue_5))
  (bind _returnvalue_9 (Math|Vector|Normalize _returnvalue_8))
  (bind _returnvalue_10 (Game|SpawnActorfromClass "/Game/GameFiles/Blueprints/Spells/BoneRipple/BP_Spell_BoneRipple.BP_Spell_BoneRipple_C" (Math|Transform|MakeTransform _returnvalue_3 (Math|Rotator|MakeRotfromX _returnvalue_9)) "Undefined" "MultiplyWithRoot" 0 0))
  (Variables|/Game/GameFiles/Blueprints/Spells/BoneRipple/BP_Spell_BoneRipple.BP_Spell_BoneRipple_C|SetDirectionVector _returnvalue_10 (* _returnvalue_9 2.5e+02)))

(event EventBeginPlay
  (bind _asbp_default_man (Utilities|Casting|CastToBP_DefaultMan (Game|GetPlayerCharacter 0)))
  (Utilities|Time|SetTimerbyEvent (delegate Custom|BoneRipple) (* (Variables|/Game/GameFiles/Blueprints/Characters/First_Char/BP_DefaultMan.BP_DefaultMan_C|GetplayerCooldown _asbp_default_man) (Variables|Default|GetCooldown)) true))

(event Collision|EventActorBeginOverlap
  (params (OtherActor :type Actor%20Object%20Reference)))

(fn ConstructionScript
  (|CallParentFunction))