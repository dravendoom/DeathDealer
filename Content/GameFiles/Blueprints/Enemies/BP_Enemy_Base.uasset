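; Base enemy Blueprint for a flipbook-animated character that faces the player, strikes in melee and drops XP on death.
; A looping timer started on BeginPlay compares X positions with the player and flips the actor left or right.
; AttackEvent plays the attack flipbook, then after a short delay restores Skeleton_Run, damages an overlapping player and calls the attack-end relayer on a hit.
; AnyDamage reduces Health, spawning BP_EXP_Orb and destroying the actor when depleted.
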(event Custom|CheckDirection
  ;[1 1 1] Orient Left/Right
  (if (> (.X (Math|Vector|BreakVector (Transformation|GetActorLocation (Game|GetPlayerCharacter 0)))) (.X (Math|Vector|BreakVector (Transformation|GetActorLocation self))))
    (Transformation|SetActorRotation "0, 0, 0" true)
    (else
      (Transformation|SetActorRotation "0.000000,180.000000,0.000000" true))))

(event Custom|AttackEvent
  (bind _self self)
  (bind _playercharacter (Variables|Default|GetPlayerCharacter))
  (Sprite|SetFlipbook (Variables|Default|GetFlipBook) (Variables|Default|GetattackFlipBook))
  (Utilities|FlowControl|Delay 0.2)
  (if (Utilities|IsValid _playercharacter)
    (Sprite|SetFlipbook (Variables|Default|GetFlipBook) "/Game/GameFiles/Sprites/Enemies/Skeleton/Skeleton_Run.Skeleton_Run")
    (if (Collision|IsOverlappingActor (Variables|Default|GetMeleeStrike) _playercharacter :!class /Script/Engine.PrimitiveComponent)
      (Game|Damage|ApplyDamage (Variables|Default|GetPlayerCharacter) 1e+01 (Pawn|GetController _self) _self "/Script/Engine.DamageType")
      (Default|CallAttackEndRelayer))))

(event Game|Damage|EventAnyDamage
  (params (Damage :type Float%20%28single-precision%29) (DamageType :type Damage%20Type%20Object%20Reference) (InstigatedBy :type Controller%20Object%20Reference) (DamageCauser :type Actor%20Object%20Reference))
  (bind _output_get (Variables|Default|SetHealth (- (Variables|Default|GetHealth) Damage)))
  (if (< _output_get 1.0)
    (Game|SpawnActorfromClass "/Game/GameFiles/Blueprints/Pawns/BP_EXP_Orb.BP_EXP_Orb_C" (Math|Transform|MakeTransform (Transformation|GetActorLocation self) "0, 0, 0" "2.000000,2.000000,2.000000") "Undefined" "MultiplyWithRoot" 0 0)
    (Actor|DestroyActor)))

(event EventBeginPlay
  (bind _returnvalue (Game|GetPlayerCharacter 0))
  (if (Utilities|IsValid _returnvalue)
    ;[1 1 1] Orient Left/Right
    (Variables|Default|SetPlayerCharacter _returnvalue)
    (Transformation|SetActorRotation "0, 0, 0")
    (Utilities|Time|SetTimerbyEvent (delegate Custom|CheckDirection) 0.01 true)))

(fn ConstructionScript)