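; Skeleton mage enemy that casts a skull spell when the player character comes within range.
; BeginPlay runs the parent setup, then overrides health, uses the necromancer move flipbook for both run and attack, and picks a mid-tier XP orb.
; SpellRange overlap with BP_DefaultMan spawns one BP_SkullSpell at the mage's location with zero rotation, owned by the mage, with no repeat timer.
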(event OnComponentBeginOverlap(SpellRange)
  (params (OverlappedComponent :type Primitive%20Component%20Object%20Reference) (OtherActor :type Actor%20Object%20Reference) (OtherComp :type Primitive%20Component%20Object%20Reference) (OtherBodyIndex :type Integer) (bFromSweep :type Boolean) (SweepResult :type Hit%20Result%20Structure%20%28by%20ref%29))
  (Utilities|Casting|CastToBP_DefaultMan OtherActor)
  (CallFunction|CastSpell))

(event Custom|Cast%20Spell
  (bind _self self)
  (Game|SpawnActorfromClass "/Game/GameFiles/Blueprints/Spells/Enemies/BP_SkullSpell.BP_SkullSpell_C" (Math|Transform|MakeTransform (Transformation|GetActorLocation _self)) "Undefined" "MultiplyWithRoot" _self 0))

(event EventBeginPlay
  (|CallParentFunction)
  (Variables|Default|SetHealth 5e+02)
  (Variables|Default|SetattackFlipBook "/Game/GameFiles/Sprites/Enemies/Necromancer/NecroMove.NecroMove")
  (Variables|Default|SetrunFlipBook "/Game/GameFiles/Sprites/Enemies/Necromancer/NecroMove.NecroMove")
  (Variables|Default|SetxpOrbType "/Game/GameFiles/Blueprints/Pawns/BP_XP_Mid.BP_XP_Mid_C"))

(event Collision|EventActorBeginOverlap
  (params (OtherActor :type Actor%20Object%20Reference)))

(event EventTick
  (params (DeltaSeconds :type Float%20%28single-precision%29)))

(fn ConstructionScript
  (|CallParentFunction))