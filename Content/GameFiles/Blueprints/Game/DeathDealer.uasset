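; DeathDealer is a game director Blueprint that spawns enemy waves around the player and presents spell choices on level-up.
; BeginPlay shows the cursor, fills a wave struct array and starts a looping CallWave timer from the first entry's frequency.
; CallWave spawns enemies at random angles a set distance from the player, uses a Delay for the second type, and advances the wave index.
; OnPlayerLevelUp creates or reuses the BP_LevelUpSpells widget with three spell selections.
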(event Custom|CallWave
  (bind _returnvalue (Game|GetPlayerCharacter 0))
  (bind _returnvalue_2 (Transformation|GetActorLocation _returnvalue))
  (bind (_x _y) (Math|Vector|BreakVector _returnvalue_2))
  (for _index (range 0 (.SpawnCount (Utilities|Struct|BreakBP_WaveStruct (Utilities|Array|Get(acopy) (Variables|Default|GetWaveStruct) (Variables|Default|GetWaveIndex)))))
    (bind _output_get (Variables|Default|SetrandomDegree (Math|Random|RandomFloatinRange 0.0 3.6e+02)))
    (Game|SpawnActorfromClass (.EnemyType (Utilities|Struct|BreakBP_WaveStruct (Utilities|Array|Get(acopy) (Variables|Default|GetWaveStruct) (Variables|Default|GetWaveIndex)))) (Math|Transform|MakeTransform (+ (+ (* (Variables|Default|GetDistance) (Math|Vector2D|Normalize2D (Math|Vector2D|MakeVector2D (Math|Trig|Cos(Radians) (Math|Trig|DegreesToRadians _output_get)) (Math|Trig|Sin(Radians) (Math|Trig|DegreesToRadians _output_get))))) (Math|Vector2D|MakeVector2D _x _y)) "0.000000,0.000000,69.000000")) "Undefined" "MultiplyWithRoot" 0 0)
    (Utilities|FlowControl|Delay 0.5)
    (Game|SpawnActorfromClass (.EnemyType2 (Utilities|Struct|BreakBP_WaveStruct (Utilities|Array|Get(acopy) (Variables|Default|GetWaveStruct) (Variables|Default|GetWaveIndex)))) (Math|Transform|MakeTransform (+ (+ (* (Variables|Default|GetDistance) (Math|Vector2D|Normalize2D (Math|Vector2D|MakeVector2D (Math|Trig|Cos(Radians) (Math|Trig|DegreesToRadians _output_get)) (Math|Trig|Sin(Radians) (Math|Trig|DegreesToRadians _output_get))))) (Math|Vector2D|MakeVector2D _x _y)) "0.000000,0.000000,69.000000")) "Undefined" "MultiplyWithRoot" 0 0))
  (bind _output_get_2 (Variables|Default|SetCurrentWavesLeft (- (Variables|Default|GetCurrentWavesLeft) 1)))
  (if (not (>= _output_get_2 0))
    (Variables|Default|SetWaveIndex (+ 1 (Variables|Default|GetWaveIndex)))
    (Variables|Default|SetCurrentWavesLeft (.WavesUntilEnd (Utilities|Struct|BreakBP_WaveStruct (Utilities|Array|Get(acopy) (Variables|Default|GetWaveStruct) (Variables|Default|GetWaveIndex)))))))

(event Custom|OnPlayerLevelUp
  (params (PlayerLevel :type Integer%20%28by%20ref%29))
  (if (Variables|Default|GetLevelUpWidgetCreated?)
    (Widget|SetVisibility (Variables|/Game/GameFiles/Blueprints/UI/BP_LevelUpSpells.BP_LevelUpSpells_C|GetCanvasPanel_63 (Variables|Default|GetLevelUpUI)) "Visible")
    (Widget|SetIsEnabled (Variables|/Game/GameFiles/Blueprints/UI/BP_LevelUpSpells.BP_LevelUpSpells_C|GetCanvasPanel_63 (Variables|Default|GetLevelUpUI)) true)
    (Default|SelectSpells (stale _output_get))
    (Default|SelectSpells (stale _output_get) "(X=350.000000,Y=0.000000)")
    (Default|SelectSpells (stale _output_get) "(X=700.000000,Y=0.000000)")
    (UserInterface|Viewport|AddtoViewport (stale _output_get) 0)
    (else
      (bind _returnvalue (UserInterface|CreateWidget "/Game/GameFiles/Blueprints/UI/BP_LevelUpSpells.BP_LevelUpSpells_C" (Game|GetPlayerController 0)))
      (bind _output_get (Variables|Default|SetLevelUpUI _returnvalue))
      (Default|BindButtons _output_get)
      (Default|SelectSpells _output_get)
      (Default|SelectSpells _output_get "(X=350.000000,Y=0.000000)")
      (Default|SelectSpells _output_get "(X=700.000000,Y=0.000000)")
      (UserInterface|Viewport|AddtoViewport _output_get 0)
      (Variables|Default|SetLevelUpWidgetCreated? true))))

(event EventBeginPlay
  (bind _skeleton (Variables|Default|GetSkeleton))
  (bind _skeletonmage (Variables|Default|GetSkeletonMage))
  (Variables|/Script/Engine.PlayerController|SetbShowMouseCursor (Game|GetPlayerController 0) true)
  (Variables|Default|SetWaveStruct (Utilities|Array|MakeArray (Utilities|Struct|MakeBP_WaveStruct _skeleton 4 2 4 _skeletonmage 0 0 0 0) (Utilities|Struct|MakeBP_WaveStruct _skeleton 3 2 10 _skeletonmage 0 0 0 0) (Utilities|Struct|MakeBP_WaveStruct _skeleton 2 4 10 _skeletonmage 0 0 0 0) "" "" "" "" "" "" "" ""))
  (Variables|Default|SetCurrentWavesLeft (.WavesUntilEnd (Utilities|Struct|BreakBP_WaveStruct (Utilities|Array|Get(acopy) (Variables|Default|GetWaveStruct) (Variables|Default|GetWaveIndex)))))
  (Utilities|Time|SetTimerbyEvent (delegate Custom|CallWave) (Math|Conversions|ToFloat(Integer) (.WaveFrequency (Utilities|Struct|BreakBP_WaveStruct (Utilities|Array|Get(acopy) (Variables|Default|GetWaveStruct) (Variables|Default|GetWaveIndex))))) true))

(fn ConstructionScript)